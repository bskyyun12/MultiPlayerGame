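; BP_ReplicationTest is a placeable test actor that moves back and forth between its starting location and a target point, apparently to exercise network replication.
; BeginPlay caches the actor location and the world location of the TargetLocation component as endpoints.
; On Tick, only the authority advances time scaled by TravelTime and sets the location with a cosine-eased lerp, producing a smooth endless ping-pong without sweeping.
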(event `self.ReceiveBeginPlay`
  (set `self.StartPosition` (`self.K2_GetActorLocation`))
  (set `self.TargetPosition` (`SceneComponent.K2_GetComponentLocation` (`self.TargetLocation`))))

(event `self.ReceiveTick`
  (params (DeltaSeconds :type "Float (single-precision)"))
  (if (`self.HasAuthority`)
    (bind _output_get (set `self.Time` (+ (`self.Time`) (/ DeltaSeconds (`self.TravelTime`)))))
    (`self.K2_SetActorLocation` (`KismetMathLibrary.VLerp` (`self.StartPosition`) (`self.TargetPosition`) (/ (+ (* (`KismetMathLibrary.Cos` (`KismetMathLibrary.MultiplyByPi` _output_get)) -1.0) 1.0) 2.0)))))

(fn `UserConstructionScript`)