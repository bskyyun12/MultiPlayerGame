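; BP_AICharacter is an AI-controlled character that spawns a weapon at BeginPlay and attaches it to the mesh's GripPoint socket.
; Its events set walk speed by AI state, from Passive to Attacking, and forward fire requests to the weapon.
; When its HealthComponent reports death, the mesh switches to ragdoll physics, capsule collision is disabled and the AI controller's brain logic stops.
; Simple getters expose death status, non-player identity, weapon and patrol.
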(event `self.ReceiveBeginPlay`
  ;[1 1 1] BeginPlay
  ;[1 1 1] Spawn weapon
  (bind _returnvalue (`|SpawnActorFromClass` (`self.WeaponClass`) (`KismetMathLibrary.MakeTransform` (0.0 0.0 0.0)) "AlwaysSpawn" "OverrideRootScale" self self))
  (bind _output_get (set `self.Weapon` _returnvalue))
  (`self.K2_AttachToComponent` _output_get (`self.Mesh`) "GripPoint" "SnapToTarget" "SnapToTarget" "KeepWorld" true))

(event `self.HealthComponent.OnDied`
  (bind _mesh (`self.Mesh`))
  ;[1 1 1] On Death
  (`PrimitiveComponent.SetCollisionProfileName` _mesh "Ragdoll" true)
  (`SkeletalMeshComponent.SetAllBodiesSimulatePhysics` _mesh true)
  (`PrimitiveComponent.WakeAllRigidBodies` _mesh)
  (`PrimitiveComponent.SetCollisionEnabled` (`self.CapsuleComponent`) "NoCollision")
  (`BrainComponent.StopLogic` (`AIController.BrainComponent` (`AIBlueprintHelperLibrary.GetAIController` self)) "Dead"))

(event `/Game/PerceptiveAI/Core/BPI_AIHelper.NotifyStateChanged`
  (params (State :type "/Game/PerceptiveAI/Characters/AI/ECombatState Enum" :default "NewEnumerator0")))

(event `/Game/PerceptiveAI/Core/BPI_AIHelper.ModifyMovementSpeed`
  (params (State :type "/Game/PerceptiveAI/Characters/AI/ECombatState Enum" :default "NewEnumerator0"))
  (set `CharacterMovementComponent.MaxWalkSpeed` (select `/Game/PerceptiveAI/Characters/AI/ECombatState` State :`NewEnumerator0` 160.0 :`NewEnumerator1` 250.0 :`NewEnumerator2` 400.0 :`NewEnumerator3` 600.0 :!type "Float (single-precision)") (`self.CharacterMovement`)))

(event `/Game/PerceptiveAI/Core/BPI_AIHelper.TryShootEquippedWeapon`
  ;[1 1 1] Try Shoot Equipped Weapon
  (bind _weapon (`self.Weapon`)
    (:`then`
      (`/Game/PerceptiveAI/Core/BP_WeaponBase.OnFireRequested` _weapon))
    (:`else`
      (`KismetSystemLibrary.PrintString` (`KismetStringLibrary.Concat_StrStr` (`KismetSystemLibrary.GetDisplayName` self) ": Weapon is not vaild.") true true (struct :`R` 1.0 :`B` 0.009094 :`A` 1.0) 5.0))))

(fn `GetPatrol`
  (returns (Patrol :type "/Game/PerceptiveAI/Characters/AI/BP_Patrol Object Reference"))
  (return (`self.Patrol`)))

(fn `GetWeapon`
  (returns (Weapon :type "/Game/PerceptiveAI/Core/BP_WeaponBase Object Reference"))
  (return (`self.Weapon`)))

(fn `IsDead`
  (returns (IsDead :type Boolean))
  (return (`/Game/PerceptiveAI/BP_HealthComponent.IsDead` (`self.HealthComponent`))))

(fn `IsPlayer`
  (returns (IsPlayer :type Boolean))
  (return false))

(fn `UserConstructionScript`)