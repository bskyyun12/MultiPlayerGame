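; BP_BulletBase is a base bullet actor for player and AI shooters, replicated when it has authority.
; On BeginPlay it asks its owner's owner whether it is a player, then gives its box the PlayerProjectile or AIProjectile collision profile.
; On hit it applies damage, makes noise using the impact's normal impulse as location, draws a brief debug point and destroys itself.
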(event `self.ReceiveBeginPlay`
  (bind _returnvalue (`self.HasAuthority`))
  (bind _box (`self.Box`))
  (`|ExecutionSequence`
    (:`then_0`
      (`self.SetReplicates` _returnvalue)
      (`self.SetReplicateMovement` _returnvalue))
    (:`then_1`
      (if (`self.IsFromPlayer`)
        (`PrimitiveComponent.SetCollisionProfileName` _box "PlayerProjectile" true)
        (else
          (`PrimitiveComponent.SetCollisionProfileName` _box "AIProjectile" true))))))

(event `self.Box.OnComponentHit`
  (params (HitComponent :type "PrimitiveComponent Object Reference") (OtherActor :type "Actor Object Reference") (OtherComp :type "PrimitiveComponent Object Reference") (NormalImpulse :type "Vector Structure") (Hit :type "HitResult Structure (by ref)"))
  (`GameplayStatics.ApplyDamage` OtherActor (`self.Damage`) null self "/Script/Engine.DamageType")
  (`self.MakeNoise` 1.0 null NormalImpulse)
  (`KismetSystemLibrary.DrawDebugPoint` (`.Location` (`GameplayStatics.BreakHitResult` Hit)) 10.0 (struct :`R` 1.0 :`B` 0.022914 :`A` 1.0) 0.2)
  (`self.K2_DestroyActor`))

(fn `IsFromPlayer`
  (returns (IsFromPlayer :type Boolean))
  (bind _isplayer (message `/Game/PerceptiveAI/Core/BPI_AIHelper.IsPlayer` (`self.GetOwner` (`self.GetOwner`))))
  (return _isplayer))

(fn `UserConstructionScript`)